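; Actor component for a player character that grants an item when a specific feat is learned.
; Five seconds after BeginPlay it binds to the feat inventory's item-added signal, the delay avoiding reactions to feats loaded from the game database at start.
; When an added feat matches the configured template ID, it spawns the configured item into the backpack's first free slot.
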(event Custom|Event%20AddFeat
  (params (index :type Integer) (item :type Game%20Item%20Object%20Reference) (srcInventory :type Item%20Inventory%20Object%20Reference) (srcIndex :type Integer))
  (bind _asfeat_item (Utilities|Casting|CastToFeatItem item))
  (if (== (Variables|/Script/ConanSandbox.GameItem|GetTemplateID _asfeat_item) (Variables|Default|GetFeatToListenFor))
    (bind _returnvalue (Class|GameItemSpawner|SpawnGameItem (Variables|Default|GetItemToSpawnForFeat)))
    (bind _asbase_player_char (Utilities|Casting|CastToBasePlayerChar (Components|GetOwner)))
    (Class|ItemInventory|AddItem (Variables|/Game/Characters/BasePlayerChar.BasePlayerChar_C|GetBackpackInventory _asbase_player_char) _returnvalue (Class|ItemInventory|GetFirstFreeIndex (Variables|/Game/Characters/BasePlayerChar.BasePlayerChar_C|GetBackpackInventory _asbase_player_char) false))))

(event EventBeginPlay
  ;[1 1 1] hack: high delay because the gamestart also adds the feats from the game.db to the inventory
  (Utilities|FlowControl|Delay 5.0)
  (bind _asbase_player_char (Utilities|Casting|CastToBasePlayerChar (Components|GetOwner)))
  (EventDispatchers|BindEventtoSignalItemAdded (Variables|/Game/Characters/BasePlayerChar.BasePlayerChar_C|GetFeatInventory _asbase_player_char) (delegate Custom|Event%20AddFeat)))