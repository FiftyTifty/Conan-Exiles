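; Stackable Sunder Armor debuff component that lowers the owning character's Armor and NaturalArmor.
; On start and stack changes it writes a Multiply stat modifier of one minus stacks times ArmorDebuffPercentage, capping adjusted stacks at StackSizeMax before calling the parent.
; Clearing writes the multiplier back to 1.0.
; The effect description labels that remaining multiplier as the percent reduction, without converting it.
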(event EventBeginPlay)

(event EventTick
  (params (DeltaSeconds :type Float%20%28single-precision%29)))

(event EventAdjustStackSize
  (params (StackAdjustment :type Integer))
  (bind _armor_debuff_percentage (Variables|Default|GetArmor%20Debuff%20Percentage))
  (bind _owningcharacter (Variables|Default|GetOwningCharacter))
  (bind _stacksize (Variables|Default|GetStackSize))
  (bind _stacksizemax (Variables|Default|GetStackSizeMax))
  (bind _returnvalue (+ _stacksize StackAdjustment))
  (bind _returnvalue_2 (Math|Integer|Min(Integer) _returnvalue _stacksizemax))
  (bind _returnvalue_3 (* _returnvalue_2 _armor_debuff_percentage))
  (bind _returnvalue_4 (- 1.0 _returnvalue_3))
  (Class|ConanCharacter|AddFloatStatModifier _owningcharacter "Armor" "Buff" "Multiply" _returnvalue_4 "Replace")
  (Class|ConanCharacter|AddFloatStatModifier _owningcharacter "NaturalArmor" "Buff" "Multiply" _returnvalue_4 "Replace")
  (|CallParentFunction StackAdjustment))

(event EventGameplayEffecttoApplyonBuffStart
  (bind _owningcharacter (Variables|Default|GetOwningCharacter))
  (bind _stacksize (Variables|Default|GetStackSize))
  (bind _armor_debuff_percentage (Variables|Default|GetArmor%20Debuff%20Percentage))
  (bind _returnvalue (* _stacksize _armor_debuff_percentage))
  (bind _returnvalue_2 (- 1.0 _returnvalue))
  (Class|ConanCharacter|AddFloatStatModifier _owningcharacter "Armor" "Buff" "Multiply" _returnvalue_2 "Replace")
  (Class|ConanCharacter|AddFloatStatModifier _owningcharacter "NaturalArmor" "Buff" "Multiply" _returnvalue_2 "Replace"))

(event EventGameplayEffecttoApplyonBuffCleared
  (bind _owningcharacter (Variables|Default|GetOwningCharacter))
  (Class|ConanCharacter|AddFloatStatModifier _owningcharacter "Armor" "Buff" "Multiply" 1.0 "Replace")
  (Class|ConanCharacter|AddFloatStatModifier _owningcharacter "NaturalArmor" "Buff" "Multiply" 1.0 "Replace"))

(fn GetEffectDescription
  (return (Utilities|Text|FormatText "Armor reduced by {ArmorReduction}%" (- 1.0 (* (Variables|Default|GetStackSize) (Variables|Default|GetArmor%20Debuff%20Percentage))))))